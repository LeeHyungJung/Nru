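; BP_NruChar_Ally is an ally character Blueprint that extends a parent character class.
; Its construction script runs the parent's, then tags the actor as a Character type with the placeholder name "Dummy".
; It also casts the movement component to ForwardMovementComponent and sets its move direction along positive X.
; BeginPlay runs the parent logic and spawns the default controller, while Tick only calls the parent.
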(event EventBeginPlay
  (|CallParentFunction)
  (Pawn|SpawnDefaultController))

(event EventActorBeginOverlap
  (params (OtherActor :type Actor%20Object%20Reference)))

(event EventTick
  (params (DeltaSeconds :type Float%20%28single-precision%29))
  (|CallParentFunction DeltaSeconds))

(fn ConstructionScript
  (|CallParentFunction)
  (Variables|Default|SetTypeEnum "Character")
  (Variables|Default|SetCharName "Dummy")
  (bind _asforward_movement_component (Utilities|Casting|CastToForwardMovementComponent (Variables|Character|GetCharacterMovement)))
  (Variables|/Script/NruDemo.ForwardMovementComponent|SetMoveDirection _asforward_movement_component "1.000000, 0, 0"))