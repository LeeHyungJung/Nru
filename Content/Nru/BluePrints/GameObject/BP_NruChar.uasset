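; BP_NruChar is a base game character with HP shown as text, destroyed when HP runs out.
; Each tick it trails its owner's follow point through a custom ForwardMovementComponent, stopping when the owner stops or it gets ahead, with timelines scaling walk speed to catch up.
; Capsule hits against a different type throw it back and deal head-butt damage, triggering a GameMode attack camera effect for the Character type.
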(event OnComponentHit(CapsuleComponent)
  (params (OtherActor :type Actor%20Object%20Reference) (OtherComp :type Primitive%20Component%20Object%20Reference) (NormalImpulse :type Vector) (Hit :type Hit%20Result%20Structure%20%28by%20ref%29))
  (bind _asbp_nru_char (Utilities|Casting|CastToBP_NruChar OtherActor))
  (if (Utilities|Enum|NotEqual(Enum) (Variables|/Script/NruDemo.NruDemoCharacter|GetTypeEnum _asbp_nru_char) (Variables|/Script/NruDemo.NruDemoCharacter|GetTypeEnum self))
    (bind _asforward_movement_component (CallFunction|GetForwardMovementComp self))
    (Class|ForwardMovementComponent|OnThrowBack _asforward_movement_component (Math|Vector|MakeVector (.X (Math|Vector|BreakVector (Class|KismetMathLibrary|GetDirectionVector (Math|Vector|GetForwardVector (Transformation|GetWorldRotation (Variables|Default|GetCapsuleComponent))) (Math|Vector|GetForwardVector (Transformation|GetWorldRotation (Variables|/Script/Engine.Character|GetCapsuleComponent _asbp_nru_char)))))) 0.7 0.7) 50000)
    (CallFunction|AttackHeadButt _asbp_nru_char)
    (switch Utilities|FlowControl|Switch|SwitchonETypeEnum (Variables|Default|GetTypeEnum)
      (:Character
        (bind _asbp_nru_game_mode (Utilities|Casting|CastToBP_NruGameMode (Game|GetGameMode)))
        (Default|BeginAttackCameraEffect _asbp_nru_game_mode self 0.5 0.5)))))

(event EventBeginPlay)

(event EventActorBeginOverlap
  (params (OtherActor :type Actor%20Object%20Reference)))

(event EventTick
  (params (DeltaSeconds :type Float%20%28single-precision%29))
  (if (<= (Variables|Property|GetHP) 0.0)
    (Actor|DestroyActor)
    (else
      (CallFunction|RenderHP)
      (|FollowOwnerChar DeltaSeconds))))

(fn ConstructionScript
  (Variables|Default|SetCharName "Base")
  (bind _asforward_movement_component (CallFunction|GetForwardMovementComp self))
  (Variables|Property|SetCharSpeed (Variables|/Script/Engine.CharacterMovementComponent|GetMaxWalkSpeed _asforward_movement_component)))

(fn GetbeMoveDirection
  (bind _valid (CallFunction|CheckFollowPosition))
  (if _valid
    (return (Class|KismetMathLibrary|GetDirectionVector (Transformation|GetActorLocation) (Transformation|GetWorldLocation (Variables|NruCharacter|GetFollowPosition))))
    (else
      (return (Math|Vector|MakeVector 0.0 0.0 0.0)))))

(fn CheckFollowPosition
  (return (!= (Variables|NruCharacter|GetFollowPosition) 0)))

(fn CheckOwnerChar
  (return (!= (Variables|Follow|GetCharOwner) 0)))

(fn GetForwardMovementComp
  (params (Nru :type Nru%20Demo%20Character%20Object%20Reference))
  (bind _asforward_movement_component (Utilities|Casting|CastToForwardMovementComponent (Pawn|GetMovementComponent Nru))
    (:then
      _)
    (:CastFailed
      _))
  (return _asforward_movement_component))

(fn IsOwnerStop
  (bind _asforward_movement_component (CallFunction|GetForwardMovementComp (Variables|Follow|GetCharOwner)))
  (return (== (.X (Math|Vector|BreakVector (Variables|/Script/Engine.MovementComponent|GetVelocity _asforward_movement_component))) 0.0)))

(fn GetFollowPointDist
  (return (Math|Vector|VectorLengthSquared (- (Transformation|GetWorldLocation (Variables|NruCharacter|GetFollowPosition)) (Transformation|GetActorLocation)))))

(fn MultiplyVelocity
  (params (A :type Float%20%28single-precision%29))
  (bind _asforward_movement_component (CallFunction|GetForwardMovementComp self))
  (Variables|/Script/Engine.CharacterMovementComponent|SetMaxWalkSpeed _asforward_movement_component (* A (Variables|Property|GetCharSpeed)))
  (return))

(fn AttackHeadButt
  (params (In%20TargetBP :type BP%20Nru%20Char%20Object%20Reference))
  (CallFunction|AddDamage In%20TargetBP (Variables|Property|GetDamage))
  (return 0))

(fn AddDamage
  (params (float :type Float%20%28single-precision%29))
  (Variables|Property|SetHP (- (Variables|Property|GetHP) float)))

(fn RenderHP
  (Rendering|Components|TextRender|SetText (Variables|Default|GetTextComponent) (Utilities|Text|ToText(Float) (Variables|Property|GetHP) "HalfToEven"))
  (return))