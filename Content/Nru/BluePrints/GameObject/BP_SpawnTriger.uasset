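; One-shot spawn trigger actor that tells the Nru game mode when the main player character enters it.
; On actor overlap, it casts the other actor to BP_NruChar_Main and passes its configured volume name to the game mode's NotiySpawn.
; A Dirty flag, set after the first notification, blocks repeat triggers.
; A small helper graph fetches and null-checks the game mode, which receives the spawn request.
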(event EventBeginPlay)

(event EventActorBeginOverlap
  (params (OtherActor :type Actor%20Object%20Reference))
  (if (not (Variables|Default|GetDirty))
    (Utilities|Casting|CastToBP_NruChar_Main OtherActor)
    (bind _nrumode (Utilities|GETNRUGAMEMODE))
    (Class|NruDemoGameMode|NotiySpawn _nrumode (Variables|Spawn|GetNotiyVolumeName))
    (Variables|Default|SetDirty true)))

(event EventTick
  (params (DeltaSeconds :type Float%20%28single-precision%29)))

(fn ConstructionScript)