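; BP_MissileAction is a projectile action object that damages and knocks back enemy characters it hits.
; On BeginPlay it reads Damage and Force from a data table row keyed by its Level.
; On sphere hit, if the struck BP_NruChar differs in type from the owning character, it throws it back along the sphere's forward via ForwardMovementComponent, ignores it for further movement collision, then applies damage.
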(event OnComponentHit(Sphere)
  (params (OtherActor :type Actor%20Object%20Reference) (OtherComp :type Primitive%20Component%20Object%20Reference) (NormalImpulse :type Vector) (Hit :type Hit%20Result%20Structure%20%28by%20ref%29))
  (bind _asbp_nru_char (Utilities|Casting|CastToBP_NruChar OtherActor))
  (bind _asbp_nru_char_2 (Utilities|Casting|CastToBP_NruChar (Components|GetOwner)))
  (if (and (Utilities|Enum|NotEqual(Enum) (Variables|/Script/NruDemo.NruDemoCharacter|GetTypeEnum _asbp_nru_char) (Variables|/Script/NruDemo.NruDemoCharacter|GetTypeEnum _asbp_nru_char_2)) (!= _asbp_nru_char_2 _asbp_nru_char))
    (bind _asforward_movement_component (Utilities|Casting|CastToForwardMovementComponent (Pawn|GetMovementComponent _asbp_nru_char)))
    (Class|ForwardMovementComponent|OnThrowBack _asforward_movement_component (Math|Vector|GetForwardVector (Transformation|GetWorldRotation (Variables|Default|GetSphere))) (Variables|Default|GetForce))
    (Collision|IgnoreActorwhenMoving (Variables|/Script/Engine.MovementComponent|GetUpdatedPrimitive (Variables|Default|GetProjectileMovement)) OtherActor true)
    (Default|AddDamage _asbp_nru_char (Math|Conversions|ToFloat(Integer) (Variables|Default|GetDamage)))))

(event EventBeginPlay
  (bind _returnvalue (Utilities|GetDataTableRow "/Game/Nru/Data/Action/DummyActionDataTable.DummyActionDataTable" (Utilities|String|StringToName (Utilities|String|ToString(Integer) (Variables|Default|GetLevel))))
    (:then
      (Variables|Default|SetDamage (.Damage (Utilities|Struct|BreakDummyActionObjectData _returnvalue)))
      (Variables|Default|SetForce (.Force (Utilities|Struct|BreakDummyActionObjectData _returnvalue))))))

(event EventActorBeginOverlap
  (params (OtherActor :type Actor%20Object%20Reference)))

(event EventTick
  (params (DeltaSeconds :type Float%20%28single-precision%29)))

(fn ConstructionScript)